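; BP_Tile is one segment of an infinite terrain, populating itself on BeginPlay with randomly placed stairs and boxes through PlaceActors.
; A forward barrier turns green and drops collision while the player overlaps its trigger, then locks red again on exit.
; When the player enters the destroy trigger, the tile destroys itself and asks InfiniteTerrainGameMode to create a new tile.
; GetAttachLocation exposes an arrow's transform as an attach point.
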(event `self.BarrierTrigger.OnComponentBeginOverlap`
  (params (OverlappedComponent :type "PrimitiveComponent Object Reference") (OtherActor :type "Actor Object Reference") (OtherComp :type "PrimitiveComponent Object Reference") (OtherBodyIndex :type Integer) (bFromSweep :type Boolean) (SweepResult :type "HitResult Structure (by ref)"))
  (`self.IsPlayerActor` OtherActor
    (:`true`
      (`self.UnlockBarrier`))))

(event `self.BarrierTrigger.OnComponentEndOverlap`
  (params (OverlappedComponent :type "PrimitiveComponent Object Reference") (OtherActor :type "Actor Object Reference") (OtherComp :type "PrimitiveComponent Object Reference") (OtherBodyIndex :type Integer))
  (`self.IsPlayerActor` OtherActor
    (:`true`
      (`self.LockBarrier`))))

(event `self.LevelDestroyTrigger.OnComponentBeginOverlap`
  (params (OverlappedComponent :type "PrimitiveComponent Object Reference") (OtherActor :type "Actor Object Reference") (OtherComp :type "PrimitiveComponent Object Reference") (OtherBodyIndex :type Integer) (bFromSweep :type Boolean) (SweepResult :type "HitResult Structure (by ref)"))
  (`self.IsPlayerActor` OtherActor
    (:`true`
      (`self.K2_DestroyActor`)
      (bind _asinfinite_terrain_game_mode (cast `/Game/Dynamic/InfiniteTerrainGameMode` (`GameplayStatics.GetGameMode`)))
      (`/Game/Dynamic/InfiniteTerrainGameMode.CreateNewTile` _asinfinite_terrain_game_mode))))

(event `self.ReceiveBeginPlay`
  (`self.PlaceActors` "/Game/Dynamic/Terrain/Props/BP_UpStairs.BP_UpStairs_C" (make `SpawnParameters` 0 2 false 1.0 1.0 780.0))
  (`self.PlaceActors` "/Game/Dynamic/Terrain/Props/BP_Box.BP_Box_C" (make `SpawnParameters` 5 15 true 0.8 2.0 60.0 60)))

(fn `GetAttachLocation`
  (returns (`Attach Transform` :type "Transform Structure"))
  (return (`SceneComponent.K2_GetComponentToWorld` (`self.Arrow`))))

(fn `LockBarrier`
  (bind _barrier_forward (`self.Barrier_Forward`))
  (`PrimitiveComponent.SetCollisionEnabled` _barrier_forward "QueryAndPhysics")
  (`PrimitiveComponent.SetMaterial` _barrier_forward 0 "/Game/Dynamic/Terrain/MI_Barrier_Red.MI_Barrier_Red"))

(fn `UnlockBarrier`
  (bind _barrier_forward (`self.Barrier_Forward`))
  (`PrimitiveComponent.SetCollisionEnabled` _barrier_forward "NoCollision")
  (`PrimitiveComponent.SetMaterial` _barrier_forward 0 "/Game/Dynamic/Terrain/MI_Barrier_Green.MI_Barrier_Green"))

(fn `UserConstructionScript`)