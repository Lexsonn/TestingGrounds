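; Tile_BP is a terrain tile for an infinite terrain system, with a forward barrier that controls the player's passage.
; When the player enters the barrier trigger, the barrier turns green and loses collision; on leaving, it relocks red and asks InfiniteTerrainGameMode to create a new tile.
; A separate destroy trigger removes the tile when the player overlaps it.
; An Arrow component's world transform is exposed as the attach location.
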(event `self.BarrierTrigger.OnComponentBeginOverlap`
  (params (OverlappedComponent :type "PrimitiveComponent Object Reference") (OtherActor :type "Actor Object Reference") (OtherComp :type "PrimitiveComponent Object Reference") (OtherBodyIndex :type Integer) (bFromSweep :type Boolean) (SweepResult :type "HitResult Structure (by ref)"))
  (`self.IsPlayerActor` OtherActor
    (:`true`
      (`self.UnlockBarrier`))))

(event `self.BarrierTrigger.OnComponentEndOverlap`
  (params (OverlappedComponent :type "PrimitiveComponent Object Reference") (OtherActor :type "Actor Object Reference") (OtherComp :type "PrimitiveComponent Object Reference") (OtherBodyIndex :type Integer))
  (`self.IsPlayerActor` OtherActor
    (:`true`
      (`self.LockBarrier`)
      (bind _asinfinite_terrain_game_mode (cast `/Game/Dynamic/InfiniteTerrainGameMode` (`GameplayStatics.GetGameMode`)))
      (`/Game/Dynamic/InfiniteTerrainGameMode.CreateNewTile` _asinfinite_terrain_game_mode))))

(event `self.LevelDestroyTrigger.OnComponentBeginOverlap`
  (params (OverlappedComponent :type "PrimitiveComponent Object Reference") (OtherActor :type "Actor Object Reference") (OtherComp :type "PrimitiveComponent Object Reference") (OtherBodyIndex :type Integer) (bFromSweep :type Boolean) (SweepResult :type "HitResult Structure (by ref)"))
  (`self.IsPlayerActor` OtherActor
    (:`true`
      (`self.K2_DestroyActor`))))

(fn `GetAttachLocation`
  (returns (`Attach Transform` :type "Transform Structure"))
  (return (`SceneComponent.K2_GetComponentToWorld` (`self.Arrow`))))

(fn `LockBarrier`
  (bind _barrier_forward (`self.Barrier_Forward`))
  (`PrimitiveComponent.SetCollisionEnabled` _barrier_forward "QueryAndPhysics")
  (`PrimitiveComponent.SetMaterial` _barrier_forward 0 "/Game/Static/Geometry/Meshes/Red_Barrier.Red_Barrier"))

(fn `UnlockBarrier`
  (bind _barrier_forward (`self.Barrier_Forward`))
  (`PrimitiveComponent.SetCollisionEnabled` _barrier_forward "NoCollision")
  (`PrimitiveComponent.SetMaterial` _barrier_forward 0 "/Game/Static/Geometry/Meshes/Green_Barrier.Green_Barrier"))

(fn `UserConstructionScript`)