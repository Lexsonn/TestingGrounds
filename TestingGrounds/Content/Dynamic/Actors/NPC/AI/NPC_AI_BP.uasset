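; NPC AI Blueprint that drives guard behavior through the GuardBehavior behavior tree and the Patrol_Data blackboard, both started on BeginPlay.
; AI Perception updates ignore actors tagged "Enemy" and write all others to the blackboard.
; A successful sense sets the actor as FocusPoint and raises Alerted, while a lost sense clears both.
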(event `self.ReceiveBeginPlay`
  (`self.UseBlackboard` "/Game/Dynamic/Actors/NPC/AI/Patrol_Data.Patrol_Data")
  (`self.RunBehaviorTree` "/Game/Dynamic/Actors/NPC/AI/GuardBehavior.GuardBehavior"))

(event `self.AIPerception.OnTargetPerceptionUpdated`
  (params (Actor :type "Actor Object Reference") (Stimulus :type "AIStimulus Structure"))
  (bind (_age _expirationage _strength _stimuluslocation _receiverlocation _tag _bsuccessfullysensed) (break `AIStimulus` Stimulus))
  (bind _focuspoint (`self.FocusPoint`))
  (bind _blackboard (`self.Blackboard`))
  (if (not (`self.ActorHasTag` Actor "Enemy"))
    (if _bsuccessfullysensed
      (`BlackboardComponent.SetValueAsObject` _blackboard _focuspoint Actor)
      (else
        (`BlackboardComponent.SetValueAsObject` _blackboard _focuspoint null)))
    (`BlackboardComponent.SetValueAsBool` _blackboard (`self.Alerted`) _bsuccessfullysensed)))

(fn `UserConstructionScript`)