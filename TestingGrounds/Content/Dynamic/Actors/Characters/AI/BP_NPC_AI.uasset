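; BP_NPC_AI is an AI controller for guard NPCs that starts the BT_GuardBehavior tree with the BB_Patrol_Data blackboard on BeginPlay.
; AI perception updates feed ProcessPerceptionStimuli, which ignores actors tagged Enemy.
; Any other sensed actor is written to the FocusPoint blackboard key, and a failed sense of such an actor clears that key.
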(event `self.ReceiveBeginPlay`
  (`self.UseBlackboard` "/Game/Dynamic/Actors/Characters/AI/BB_Patrol_Data.BB_Patrol_Data")
  (`self.RunBehaviorTree` "/Game/Dynamic/Actors/Characters/AI/BT_GuardBehavior.BT_GuardBehavior"))

(event `self.AIPerception.OnTargetPerceptionUpdated`
  (params (Actor :type "Actor Object Reference") (Stimulus :type "AIStimulus Structure"))
  (`self.Process Perception Stimuli` Actor Stimulus))

(fn `Process Perception Stimuli`
  (params (ObjectValue :type "Actor Object Reference") (AIStimulus :type "AIStimulus Structure (by ref)"))
  (bind _focuspoint (`self.FocusPoint`))
  (bind _blackboard (`self.Blackboard`))
  (if (`self.ActorHasTag` ObjectValue "Enemy")
    _
    (elif (`.bSuccessfullySensed` (break `AIStimulus` AIStimulus))
      (`BlackboardComponent.SetValueAsObject` _blackboard _focuspoint ObjectValue)
      (else
        (`BlackboardComponent.ClearValue` _blackboard _focuspoint)))))

(fn `UserConstructionScript`)