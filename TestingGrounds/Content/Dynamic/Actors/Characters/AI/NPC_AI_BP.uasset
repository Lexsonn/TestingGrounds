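; NPC_AI_BP is the AI controller for guard NPCs, running the GuardBehavior tree on the Patrol_Data blackboard.
; AI perception updates for actors without the "Enemy" tag set the blackboard FocusPoint to that actor when sensed, or clear it when lost.
; The same sensing result drives the controlled character's Alerted and Shooting flags, so the guard shoots whenever it is alerted.
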(event `self.ReceiveBeginPlay`
  (`self.UseBlackboard` "/Game/Dynamic/Actors/Characters/AI/Patrol_Data.Patrol_Data")
  (`self.RunBehaviorTree` "/Game/Dynamic/Actors/Characters/AI/GuardBehavior.GuardBehavior"))

(event `self.AIPerception.OnTargetPerceptionUpdated`
  (params (Actor :type "Actor Object Reference") (Stimulus :type "AIStimulus Structure"))
  (bind (_age _expirationage _strength _stimuluslocation _receiverlocation _tag _bsuccessfullysensed) (break `AIStimulus` Stimulus))
  (bind _focuspoint (`self.FocusPoint`))
  (bind _blackboard (`self.Blackboard`))
  (if (not (`self.ActorHasTag` Actor "Enemy"))
    (if _bsuccessfullysensed
      (`BlackboardComponent.SetValueAsObject` _blackboard _focuspoint Actor)
      (else
        (`BlackboardComponent.SetValueAsObject` _blackboard _focuspoint null)))
    (bind _ascharacter (cast `/Game/Dynamic/Actors/Characters/Guard/Character` (`self.K2_GetPawn`)))
    (bind _output_get (set `/Game/Dynamic/Actors/Characters/Guard/Character.Alerted` _bsuccessfullysensed _ascharacter))
    (set `/Game/Dynamic/Actors/Characters/Guard/Character.Shooting` _output_get _ascharacter)))

(fn `UserConstructionScript`)