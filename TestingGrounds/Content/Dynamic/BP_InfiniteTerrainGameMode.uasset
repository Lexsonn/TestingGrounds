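; Game mode for an infinite-terrain game that spawns chained terrain tiles and tracks a score.
; On BeginPlay it populates a NavMeshBoundsVolume pool, then creates the minimum number of loaded tiles.
; CreateNewTile spawns a tile at the stored transform, hands it the shared pool, and saves its attach location as the next spawn point.
; IncreaseScore increments the score counter.
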(event `self.ReceiveBeginPlay`
  (`self.PopulateBoundsVolumePool`)
  (for _ (range 1 (+ (`self.MinLoadedLevelsAtOnce`) 1))
    (`self.CreateNewTile`)))

(fn `CreateNewTile`
  (bind _returnvalue (`|SpawnActorFromClass` "/Game/Dynamic/Terrain/BP_Tile.BP_Tile_C" (`self.NextTileTransform`) "Undefined" "OverrideRootScale" null null))
  (`Tile.SetPool` _returnvalue (`self.NavMeshBoundsVolumePool`))
  (bind _attach_transform (`/Game/Dynamic/Terrain/BP_Tile.GetAttachLocation` _returnvalue))
  (set `self.NextTileTransform` _attach_transform))

(fn `IncreaseScore`
  (`/Engine/EditorBlueprintResources/StandardMacros.IncrementInt` (`self.Score`)))

(fn `UserConstructionScript`)